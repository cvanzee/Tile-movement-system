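; Enemy bullet actor that passes damage to whatever it overlaps and expires after a set time.
; Its box overlap sends an EnemyBulletDamage message to the other actor with the damage amount, damage type and a self reference, leaving the response to the receiver.
; BeginPlay starts BulletRange, which uses the range value as a delay before destroying the bullet.
; AbsorbDisk, EnemyBulletDamage and SpecialItemCollected are empty stubs here.
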(event `self.ReceiveBeginPlay`
  (`self.Bullet Range`))

(event `self.Box.OnComponentBeginOverlap`
  (params (OverlappedComponent :type "PrimitiveComponent Object Reference") (OtherActor :type "Actor Object Reference") (OtherComp :type "PrimitiveComponent Object Reference") (OtherBodyIndex :type Integer) (bFromSweep :type Boolean) (SweepResult :type "HitResult Structure (by ref)"))
  (message `/Game/1_Mobs/BP_ENEMYattack_interface.Enemy Bullet Damage` OtherActor (`self.Bullet Damage`) self (`self.Damage Type`)))

(fn `Absorb Disk`
  (params (Neutral :type "Float (double-precision)") (`Disk Reference` :type "/Game/ThirdPersonBP/Charging_Bullet Object Reference") (Solar :type "Float (double-precision)") (Void :type "Float (double-precision)"))
  (returns (NewParam :type "Float (double-precision)"))
  (return 0.0))

(fn `Enemy Bullet Damage`
  (params (IncommingDamage :type "Float (double-precision)") (`Bullet Reference` :type "/BP_enemy_bullet Object Reference") (`Damage Type` :type Integer)))

(fn `Special Item Collected`
  (params (`Item Ref` :type "/Game/1_Mobs/Special_Item_parent Object Reference") (`Item ID` :type Integer))
  (returns (NewParam :type "/BP_enemy_bullet Object Reference"))
  (return null))

(fn `UserConstructionScript`)